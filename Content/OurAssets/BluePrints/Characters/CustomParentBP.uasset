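; CustomParentBP is a base character Blueprint for units, layered on a parent class whose BeginPlay, Tick, AttackVictim and DestroyUnit events it calls through to.
; DestroyUnit also triggers the death animation on the Pawn_Anim_BP_Parent anim instance.
; Tick toggles an idle DoOnce with no output, while attack, move and special-ability logic sits disconnected.
; CoolAbility is a placeholder that only prints a debug warning about using the default.
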(event `self.ReceiveBeginPlay`
  ;[1 1 1] default
  (`parent.ReceiveBeginPlay`))

(event `self.ReceiveTick`
  (params (DeltaSeconds :type "Float (single-precision)"))
  ;[1 1 1] default
  (`parent.ReceiveTick` DeltaSeconds)
  (if (`self.Idle`)
    (`/Engine/EditorBlueprintResources/StandardMacros.DoOnce` true :!label _label)
    (else
      (`|ExecutionSequence`
        (:`then_0`
          (goto _label :!via `Reset`))))))

(event `self.Attack Victim`
  (params (Victim :type "/Game/OurAssets/BluePrints/Characters/Unit_Parent Object Reference"))
  ;[1 1 1] default
  (`parent.Attack Victim` Victim))

(event `self.Destroy Unit`
  (params (`Anim Delay` :type "Float (single-precision)"))
  ;[1 1 1] default
  (`parent.Destroy Unit` `Anim Delay`)
  (bind _aspawn_anim_bp_parent (cast `/Game/AdvancedTurnBasedTileToolkit/Animations/Pawn_Anim_BP_Parent` (`SkeletalMeshComponent.GetAnimInstance` (`self.SkeletalMesh_0`))))
  (`/Game/AdvancedTurnBasedTileToolkit/Animations/Pawn_Anim_BP_Parent.DeathAnimation` _aspawn_anim_bp_parent))

(fn `coolAbility`
  (`KismetSystemLibrary.PrintString` "defgault cool ability... bad."))

(fn `UserConstructionScript`
  (`parent.UserConstructionScript`))