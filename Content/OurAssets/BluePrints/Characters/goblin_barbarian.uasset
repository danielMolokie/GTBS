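; Goblin barbarian unit Blueprint that extends parent unit logic with skeletal mesh animation for movement, attacks and death.
; Tick triggers the anim Blueprint's move animation, once on entering Idle and every tick otherwise, clearing its Break flag when not idle.
; Attacks play a second animation when the special ability is primed, then clear that flag.
; Death passes the mesh to the parent, while DestroyUnit plays the death animation.
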(event `self.ReceiveBeginPlay`
  (`parent.ReceiveBeginPlay`))

(event `Destroy Unit`
  (params (`Anim Delay` :type "Float (double-precision)"))
  (bind _aspawn_anim_bp_parent (cast `/Game/AdvancedTurnBasedTileToolkit/Animations/Pawn_Anim_BP_Parent` (`SkeletalMeshComponent.GetAnimInstance` (`self.SkeletalMesh_0`))))
  (`/Game/AdvancedTurnBasedTileToolkit/Animations/Pawn_Anim_BP_Parent.DeathAnimation` _aspawn_anim_bp_parent))

(event `self.ReceiveTick`
  (params (DeltaSeconds :type "Float (single-precision)"))
  (bind _asgoblin_barbarian_anim (cast `/Game/OurAssets/Animations/goblin_barbarian_anim` (`SkeletalMeshComponent.GetAnimInstance` (`self.SkeletalMesh_0`)) :!pure true))
  (`parent.ReceiveTick` DeltaSeconds)
  (if (`self.Idle`)
    (`/Engine/EditorBlueprintResources/StandardMacros.DoOnce` true :!label _label
      (:`Completed`
        _))
    (else
      (`|ExecutionSequence`
        (:`then_0`
          (goto _label :!via `Reset`))
        (:`then_1`
          (set `/Game/OurAssets/Animations/goblin_barbarian_anim.Break` false _asgoblin_barbarian_anim)))))
  (`/Game/OurAssets/Animations/goblin_barbarian_anim.MoveAnimation` _asgoblin_barbarian_anim))

(event `self.Attack Victim`
  (params (Victim :type "/Game/OurAssets/BluePrints/Characters/Unit_Parent Object Reference"))
  (`parent.Attack Victim` Victim)
  (bind _asgoblin_barbarian_anim (cast `/Game/OurAssets/Animations/goblin_barbarian_anim` (`SkeletalMeshComponent.GetAnimInstance` (`self.SkeletalMesh_0`))))
  (if (`self.specialAbilityPrimed`)
    (bind _asgoblin_barbarian_anim_2 (cast `/Game/OurAssets/Animations/goblin_barbarian_anim` (`SkeletalMeshComponent.GetAnimInstance` (`self.SkeletalMesh_0`))))
    (`/Game/OurAssets/Animations/goblin_barbarian_anim.attack2animation` _asgoblin_barbarian_anim_2)
    (`KismetSystemLibrary.PrintString` "Attack2Animation")
    (set `self.specialAbilityPrimed` false)
    (else
      (`/Game/OurAssets/Animations/goblin_barbarian_anim.AttackAnimation` _asgoblin_barbarian_anim))))

(event `self.Die`
  (params (mesh :type "SkeletalMeshComponent Object Reference"))
  (`parent.Die` (`self.SkeletalMesh_0`)))

(fn `UserConstructionScript`
  (`parent.UserConstructionScript`))