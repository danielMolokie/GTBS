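; Chef character Blueprint, a child class that drives its chef_anim animation instance from inherited movement and attack behavior.
; On Tick, while not Idle it clears the anim's Break flag and calls MoveAnimation each frame, re-arming a DoOnce.
; When Idle, that DoOnce, which starts closed, lets MoveAnimation fire only once.
; AttackVictim runs the parent logic, then randomly plays one of two attack animations.
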(event `self.ReceiveTick`
  (params (DeltaSeconds :type "Float (single-precision)"))
  (bind _aschef_anim (cast `/Game/OurAssets/Animations/chef_anim` (`SkeletalMeshComponent.GetAnimInstance` (`self.SkeletalMesh`)) :!pure true))
  (`parent.ReceiveTick` DeltaSeconds)
  (if (`self.Idle`)
    (`/Engine/EditorBlueprintResources/StandardMacros.DoOnce` true :!label _label
      (:`Completed`
        _))
    (else
      (`|ExecutionSequence`
        (:`then_0`
          (goto _label :!via `Reset`))
        (:`then_1`
          (set `/Game/OurAssets/Animations/chef_anim.Break` false _aschef_anim)))))
  (`/Game/OurAssets/Animations/chef_anim.MoveAnimation` _aschef_anim))

(event `self.Attack Victim`
  (params (Victim :type "/Game/OurAssets/BluePrints/Unit_Parent Object Reference"))
  (`parent.Attack Victim` Victim)
  (bind _aschef_anim (cast `/Game/OurAssets/Animations/chef_anim` (`SkeletalMeshComponent.GetAnimInstance` (`self.SkeletalMesh`))))
  (if (`KismetMathLibrary.RandomBool`)
    (`/Game/OurAssets/Animations/chef_anim.AttackAnimation` _aschef_anim)
    (else
      (`/Game/OurAssets/Animations/chef_anim.attack2animation` _aschef_anim))))

(fn `UserConstructionScript`
  (`parent.UserConstructionScript`))