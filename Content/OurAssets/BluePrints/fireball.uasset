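; Fireball projectile actor that flies toward a stored target position.
; Once its Begin flag is set, each Tick sets the ProjectileMovement velocity to the offset from the target times a constant, so it slows as it closes in.
; It destroys itself when horizontal speed drops below a small threshold, ignoring Z, with no hit or damage logic in this graph.
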(event `self.ReceiveTick`
  (params (DeltaSeconds :type "Float (single-precision)"))
  (bind (_returnvalue_x _returnvalue_y _returnvalue_z) (`KismetMathLibrary.BreakVector` (- (`self.positionOfUnluckySchmuck`) (`self.K2_GetActorLocation` self))))
  (if (`self.begin`)
    (bind _output_get (set `MovementComponent.Velocity` (`KismetMathLibrary.MakeVector` (* _returnvalue_x 5.0) (* _returnvalue_y 5.0) (* _returnvalue_z 5.0)) (`self.ProjectileMovement`)))
    (if (< (`KismetMathLibrary.Hypotenuse` (.x _output_get) (.y _output_get)) 1.0)
      (`self.K2_DestroyActor`))))

(fn `UserConstructionScript`)