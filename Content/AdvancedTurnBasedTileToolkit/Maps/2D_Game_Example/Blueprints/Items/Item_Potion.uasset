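; Healing potion item for the 2D example game of the Advanced Turn Based Tile Toolkit.
; On ActivateItem, if the activating unit is a 2D sprite hero, it adds HealAmount to that unit's health, capped at its maximum.
; It then updates the hero's dynamic health bar material fill, destroys itself and plays a potion sound.
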(event `self.Activate Item`
  (params (`Activating Unit` :type "/Game/AdvancedTurnBasedTileToolkit/Maps/2D_Game_Example/Blueprints/Pawns/Unit_Parent_2D Object Reference"))
  (bind _maxhealth (`/Game/OurAssets/BluePrints/Characters/Unit_Parent.MaxHealth` `Activating Unit`))
  (cast `/Game/AdvancedTurnBasedTileToolkit/Maps/2D_Game_Example/Blueprints/Pawns/Unit_2D_Sprite_Hero` `Activating Unit`)
  (bind _output_get (set `/Game/OurAssets/BluePrints/Characters/Unit_Parent.CurrentHealth` (`KismetMathLibrary.FMin` (+ (`self.Heal Amount`) (`/Game/OurAssets/BluePrints/Characters/Unit_Parent.CurrentHealth` `Activating Unit`)) _maxhealth) `Activating Unit`))
  (`MaterialInstanceDynamic.SetScalarParameterValue` (`/Game/OurAssets/BluePrints/Characters/Unit_Parent.Dynamic Health Bar Material` `Activating Unit`) "PercentFill" (/ _output_get _maxhealth))
  (`self.K2_DestroyActor`)
  (`GameplayStatics.PlaySound2D` "/Game/AdvancedTurnBasedTileToolkit/Maps/2D_Game_Example/Sound/Potion.Potion"))

(fn `UserConstructionScript`
  (`parent.UserConstructionScript`))