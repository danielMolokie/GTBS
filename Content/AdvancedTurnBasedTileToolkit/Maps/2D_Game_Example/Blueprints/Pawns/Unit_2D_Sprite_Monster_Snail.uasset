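; Snail monster unit for the tile toolkit's 2D example, protected by a shell until its health is worn down.
; Its Damage event reduces incoming damage by a flat amount while the health ratio is above a threshold, then forwards it to the parent.
; At or below that threshold it takes full damage and, once, swaps the shelled sprite for the NoShell one.
; Health is checked before the hit applies, so the swap shows on the following hit.
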(event `self.Receive Damage`
  (params (Damage :type "Float (single-precision)") (`Anim Delay` :type "Float (single-precision)"))
  (bind _returnvalue (<= (/ (`self.CurrentHealth`) (`self.MaxHealth`)) 0.7))
  (if _returnvalue
    (`|ExecutionSequence`
      (:`then_0`
        (`/Engine/EditorBlueprintResources/StandardMacros.DoOnce` false
          (:`Completed`
            (`SceneComponent.SetVisibility` (`self.PaperSprite`) false false)
            (`SceneComponent.SetVisibility` (`self.No Shell`) true false))))
      (:`then_1`
        (`parent.Receive Damage` (`KismetMathLibrary.SelectFloat` Damage (- Damage 20.0) _returnvalue) `Anim Delay` :!label _label)))
    (else
      (goto _label))))

(fn `UserConstructionScript`
  (`parent.UserConstructionScript`))